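; GQRoom is a room actor that holds navigation nodes for eight compass directions, plus named object nodes.
; The construction script packs editor-assigned direction nodes into an array indexed by direction, with lookups by direction, first available node or object display name.
; GetNextNode steps left or right from a direction to find an occupied slot, turning leftward steps into wrap-around additions because bytes are unsigned.
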(event EventBeginPlay)

(event EventActorBeginOverlap
  (params (OtherActor :type Actor%20Object%20Reference)))

(event EventTick
  (params (DeltaSeconds :type Float%20%28single-precision%29)))

(fn ConstructionScript
  (CallFunction|PopulateNodeArray))

(fn GetNodebyDirection
  (params (Direction :type Directions%20Enum))
  (bind _returnvalue (Math|Conversions|ToInteger(Byte) Direction))
  (bind _nodes (Variables|Default|GetNodes))
  (bind _item (Utilities|Array|Get(acopy) _nodes _returnvalue))
  (return _item (not (== _item 0))))

(fn PopulateNodeArray
  (Variables|Default|SetNodes (Utilities|Array|MakeArray (Variables|Default|GetNorth) (Variables|Default|GetNorth%20East) (Variables|Default|GetEast) (Variables|Default|GetSouth%20East) (Variables|Default|GetSouth) (Variables|Default|GetSouth%20West) (Variables|Default|GetWest) (Variables|Default|GetNorth%20West))))

(fn GetNextNode
  (params (Current%20Direction :type Directions%20Enum) (Left%20or%20Right :type LeftOrRight%20Enum))
  (bind _new_step_size (CallFunction|CalculateStepSize Left%20or%20Right (LocalVariables|GetStep%20Size)))
  (LocalVariables|SetStep%20Size _new_step_size)
  (for _array_element (Variables|Default|GetNodes)
    (bind _direction (CallFunction|ConvertBytetoDirection (+ Current%20Direction (LocalVariables|GetStep%20Size))))
    (bind (_node _node_exists) (CallFunction|GetNodebyDirection _direction))
    (if _node_exists
      (return _node)
      (else
        (bind _new_step_size_2 (CallFunction|CalculateStepSize Left%20or%20Right (LocalVariables|GetStep%20Size)))
        (LocalVariables|SetStep%20Size _new_step_size_2))))
  (Development|PrintString "This room seems to have no nodes in it")
  (return 0))

(fn CalculateStepSize
  (params (Selection :type LeftOrRight%20Enum) (Old%20Step%20Size :type Byte))
  (switch Utilities|FlowControl|Switch|SwitchonLeftOrRight Selection
    (:NewEnumerator0
      (return (+ Old%20Step%20Size (Math|Conversions|ToByte(Integer) (- (|GetNumEnumEntries) 1)))))
    (:NewEnumerator1
      (return (+ Old%20Step%20Size 1)))))

(fn GetAnyNode
  (bind _enumvalue (|ForEachDirections)
    (:LoopBody
      (bind (_node _node_exists) (CallFunction|GetNodebyDirection _enumvalue))
      (if _node_exists
        (return _node)))
    (:then
      (return 0))))

(fn GetObjectNode
  (params (Node%20Name :type String))
  (for _array_element (Variables|Default|GetObject%20Nodes)
    (if (Utilities|Enum|Equal(Enum) Node%20Name (Utilities|GetDisplayName _array_element))
      (return true _array_element)))
  (return false 0))