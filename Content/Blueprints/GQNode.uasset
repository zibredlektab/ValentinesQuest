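; GQNode is a node Blueprint that shows an optional UI widget while the node is entered.
; On BeginPlay it flags whether WidgetLayoutClass holds any entries and, if so, creates a widget from the first one.
; EnterNode adds that cached widget to the viewport and ExitNode removes it from its parent, both only when the flag is set.
; Debug prints reporting widget presence are left disconnected.
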(event `self.ReceiveBeginPlay`
  (bind _widget_layout_class (`self.Widget Layout Class`))
  (bind _output_get (set `self.Has Widget` (not (== (`KismetArrayLibrary.Array_Length` _widget_layout_class) 0))))
  (if _output_get
    (bind _returnvalue (`|CreateWidget` (`KismetArrayLibrary.Array_Get` _widget_layout_class)))
    (bind _output_get_2 (set `self.Widget Layout` _returnvalue))))

(event `self.ReceiveActorBeginOverlap`
  (params (OtherActor :type "Actor Object Reference")))

(event `self.ReceiveTick`
  (params (DeltaSeconds :type "Float (single-precision)")))

(fn `Enter Node`
  (`|ExecutionSequence`
    (:`then_0`
      (if (`self.Has Widget`)
        (`UserWidget.AddToViewport` (`self.Widget Layout`) 0)))))

(fn `Exit Node`
  (if (`self.Has Widget`)
    (`Widget.RemoveFromParent` (`self.Widget Layout`))))

(fn `UserConstructionScript`)