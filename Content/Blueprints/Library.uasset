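; Blueprint function library with a helper that converts a Byte into a Directions enum value.
; Values at or above the enum's entry count wrap around by repeated subtraction of that count, so any byte maps to a valid direction.
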(fn ConvertBytetoDirection
  (params (Byte :type Byte))
  (bind _returnvalue (|GetNumEnumEntries))
  (bind _output_get (LocalVariables|SetSafe%20Byte Byte))
  (while (>= _output_get (Math|Conversions|ToByte(Integer) _returnvalue))
    (bind _output_get_2 (LocalVariables|SetSafe%20Byte (- (LocalVariables|GetSafe%20Byte) (Math|Conversions|ToByte(Integer) _returnvalue)))))
  (return (Utilities|Enum|ByteToEnumDirections _output_get_2)))