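; Player controller for GarageQuest that runs node-based navigation, placing the player at static views within rooms.
; At start it creates the GQUI widget, gathers GQRoom actors and enters a starting node; turning and room changes exit and enter nodes.
; Node changes flag a GUI refresh on Tick, updating background image, debug text and left/right navigation, enabled only for room views.
; It also stores named switch states in parallel arrays.
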(event `self.ReceiveBeginPlay`
  (`|ExecutionSequence`
    (:`then_0`
      (bind _returnvalue (`|CreateWidget` "/Game/Blueprints/GQUI.GQUI_C"))
      (bind _output_get (set `self.GUI` _returnvalue))
      (`UserWidget.AddToViewport` _output_get 0))
    (:`then_1`
      (set `self.CurrentDirection` "NewEnumerator0"))
    (:`then_2`
      (`self.Populate Room Array`)
      (bind (_room _found_room) (`self.Find Room` "NewEnumerator0"))
      (if _found_room
        (set `self.CurrentRoom` _room)
        (else
          (`KismetSystemLibrary.PrintString` "Room does not exist"))))
    (:`then_3`
      (bind (_node _node_exists) (`/Game/Blueprints/GQRoom.Get Node by Direction` (`self.CurrentRoom`) (`self.CurrentDirection`)))
      (if _node_exists
        (`self.Move To Node` _node)
        (`self.Update GUI`)
        (else
          (`KismetSystemLibrary.PrintString` "Starting node does not exist"))))))

(event `self.ReceiveTick`
  (params (DeltaSeconds :type "Float (single-precision)"))
  (if (`self.GUINeedsUpdate`)
    (`self.Update GUI`)))

(fn `Find Room`
  (params (`Room to Find` :type "/Game/Blueprints/Room Enum"))
  (returns (Room :type "/Game/Blueprints/GQRoom Object Reference") (`Found Room` :type Boolean))
  (for _array_element (`self.Rooms`)
    (if (`|EnumEquality` (`/Game/Blueprints/GQRoom.Room` _array_element) `Room to Find`)
      (return _array_element true)))
  (return null false))

(fn `Get Switch State`
  (params (`Switch Name` :type String))
  (returns (`Found Switch` :type Boolean) (State :type Boolean))
  (for (_array_element _array_index) (`self.Switch Names`)
    (if (== _array_element `Switch Name`)
      (return true (`KismetArrayLibrary.Array_Get` (`self.Switches`) _array_index))))
  (return false false))

(fn `Make Debug Text`
  (returns (`Debug Text` :type Text))
  (bind _currentnode (`self.CurrentNode`))
  (return (`KismetTextLibrary.Conv_StringToText` (`KismetStringLibrary.JoinStringArray` (`|MakeArray` "Room:" (`KismetSystemLibrary.GetDisplayName` (`self.CurrentRoom`)) "| Direction:" (`|GetEnumeratorNameAsString` (`self.CurrentDirection`)) "| Node:" (`KismetSystemLibrary.GetDisplayName` _currentnode) "| Has Overlay:" (`KismetStringLibrary.Conv_BoolToString` (`/Game/Blueprints/GQNode.Has Widget` _currentnode)))))))

(fn `Move To Node`
  (params (`Node to Move to` :type "/Game/Blueprints/GQNode Object Reference"))
  (bind _currentnode (`self.CurrentNode`))
  (if (not (== _currentnode null))
    (`/Game/Blueprints/GQNode.Exit Node` _currentnode))
  (bind _output_get (set `self.CurrentNode` `Node to Move to`))
  (`/Game/Blueprints/GQNode.Enter Node` _output_get)
  (set `self.GUINeedsUpdate` true))

(fn `Move To Room`
  (params (`Room to Move to` :type "/Game/Blueprints/Room Enum"))
  (bind (_room _found_room) (`self.Find Room` `Room to Move to`))
  (if _found_room
    (bind _output_get (set `self.CurrentRoom` _room))
    (bind (_node _node_exists) (`/Game/Blueprints/GQRoom.Get Node by Direction` _output_get (`self.CurrentDirection`)))
    (if _node_exists
      (`self.Move To Node` _node)
      (else
        (bind _node_2 (`/Game/Blueprints/GQRoom.Get Any Node` (`self.CurrentRoom`)))
        (`KismetSystemLibrary.PrintString` "Moving to a random node")
        (`self.Move To Node` _node_2)))
    (else
      (`KismetSystemLibrary.PrintString` "Room does not exist"))))

(fn `Populate Room Array`
  (bind _outactors (`GameplayStatics.GetAllActorsOfClass` "/Game/Blueprints/GQRoom.GQRoom_C"))
  (set `self.Rooms` _outactors))

(fn `Set Switch State`
  (params (`Switch Name` :type String) (`New State` :type Boolean))
  (returns (`Found Switch` :type Boolean))
  (for (_array_element _array_index) (`self.Switch Names`)
    (if (== _array_element `Switch Name`)
      (`KismetArrayLibrary.Array_Set` (`self.Switches`) _array_index `New State`)
      (return true)))
  (return false))

(fn `Turn to Direction`
  (params (Direction :type "/Game/Blueprints/LeftOrRight Enum"))
  (bind _next_node (`/Game/Blueprints/GQRoom.Get Next Node` (`self.CurrentRoom`) (`self.CurrentDirection`) Direction))
  (set `self.CurrentDirection` (`/Game/Blueprints/GQNode.Direction` _next_node))
  (`self.Move To Node` _next_node))

(fn `Update GUI`
  (bind _currentnode (`self.CurrentNode`))
  (bind _gui (`self.GUI`))
  (if (not (== (`self.GUI`) null))
    (`|ExecutionSequence`
      (:`then_0`
        (`/Game/Blueprints/GQUI.SetBackgroundImage` (`self.GUI`) (`/Game/Blueprints/GQNode.View` _currentnode)))
      (:`then_1`
        (switch `/Game/Blueprints/NodeType` (`/Game/Blueprints/GQNode.Node Type` _currentnode)
          (:`NewEnumerator0`
            (set `/Game/Blueprints/GQUI.Left Right Nav Enabled` true _gui))
          (:`NewEnumerator1`
            (set `/Game/Blueprints/GQUI.Left Right Nav Enabled` false _gui :!label _label))
          (:`NewEnumerator2`
            (goto _label))))
      (:`then_2`
        (bind _debug_text (`self.Make Debug Text`))
        (set `/Game/Blueprints/GQUI.Debug Text` _debug_text (`self.GUI`)))
      (:`then_3`
        (set `self.GUINeedsUpdate` false)))))

(fn `UserConstructionScript`)