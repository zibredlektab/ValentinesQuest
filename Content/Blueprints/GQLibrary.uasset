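; GQLibrary is a Blueprint library of shared helper functions for GarageQuest.
; It creates zoom overlay and fade caption widgets from supplied content, and fetches player 0's controller cast to the game's own class.
; Conversion helpers split an integer into two digit strings with zero padding, and wrap bytes into the Directions enum range by repeated subtraction to avoid an engine crash on out-of-range values.
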(fn ConvertBytetoDirection
  (params (Byte :type Byte))
  (bind _returnvalue (|GetNumEnumEntries))
  (bind _output_get (LocalVariables|SetSafe%20Byte Byte))
  (while (>= _output_get (Math|Conversions|ToByte(Integer) _returnvalue))
    (bind _output_get_2 (LocalVariables|SetSafe%20Byte (- (LocalVariables|GetSafe%20Byte) (Math|Conversions|ToByte(Integer) _returnvalue)))))
  (return (Utilities|Enum|ByteToEnumDirections _output_get_2)))

(fn MakeZoomOverlay
  (params (Object%20Image :type Texture%202D%20Object%20Reference) (Caption :type Text))
  (bind _returnvalue (UserInterface|CreateWidget "/Game/Blueprints/ZoomIn.ZoomIn_C" (Game|GetPlayerController 0)))
  (Variables|/Game/Blueprints/ZoomIn.ZoomIn_C|SetTexture _returnvalue Object%20Image)
  (Variables|/Game/Blueprints/ZoomIn.ZoomIn_C|SetCaptionText _returnvalue Caption)
  (return _returnvalue))

(fn GetGQPlayerController
  (bind _asgarage_quest_player_controller (Utilities|Casting|CastToGarageQuest_PlayerController (Game|GetPlayerController 0)))
  (return _asgarage_quest_player_controller))

(fn InttoTwoStrings
  (params (Int :type Integer))
  (bind _returnvalue (Utilities|String|ToString(Integer) Int))
  (bind _returnvalue_2 (Utilities|String|GetCharacterArrayfromString _returnvalue))
  (if (> Int 9)
    (return (Utilities|Array|Get(acopy) _returnvalue_2) (Utilities|Array|Get(acopy) _returnvalue_2 1))
    (else
      (return "0" (Utilities|String|ToString(Integer) Int)))))

(fn MakeFadeCaption
  (params (Captions :type Array%20of%20Texts) (Should%20Fade%20Final%20Caption :type Boolean))
  (bind _returnvalue (UserInterface|CreateWidget "/Game/Blueprints/NodeLayouts/FadeCaption.FadeCaption_C"))
  (bind _output_get (LocalVariables|SetWidget _returnvalue))
  (Default|SetupFadeCaption _output_get Captions Should%20Fade%20Final%20Caption)
  (return _output_get))